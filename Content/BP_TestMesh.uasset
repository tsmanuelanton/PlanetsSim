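; BP_TestMesh is a test actor that builds a flat X-by-Y grid of unit quads on a procedural mesh in its construction script.
; Spawn clears the arrays, CreateVertex adds six unshared vertices per cell, and CreateTriangles indexes them sequentially, running one index past the end.
; The section gets no UVs, as CreateUVs is never called.
; An alternative built with CreateGridMeshWelded is left disconnected.
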(fn `CreateTriangles`
  (for _index (range (+ (`KismetArrayLibrary.Array_Length` (`self.Vertex2`)) 1))
    (`KismetSystemLibrary.PrintString` "Hello")
    (`KismetArrayLibrary.Array_Add` (`self.Triangles2`) _index)))

(fn `CreateUVs`
  (bind _uv0 (`self.UV0`))
  (`KismetArrayLibrary.Array_Add` _uv0)
  (`KismetArrayLibrary.Array_Add` _uv0 (100.0 0.0))
  (`KismetArrayLibrary.Array_Add` _uv0 (0.0 100.0)))

(fn `CreateVertex`
  (locals (TempX :type Integer) (TempY :type Integer))
  (bind _vertex2 (`self.Vertex2`))
  (bind _vertex2_2 (`self.Vertex2`))
  (bind _tempx (`local.TempX`))
  (bind _tempy (`local.TempY`))
  (bind _tempy_2 (`local.TempY`))
  (bind _returnvalue (+ _tempy 1))
  (bind _returnvalue_2 (`KismetMathLibrary.Conv_IntToDouble` (+ _tempx 1)))
  (for _index (range (`self.Y`))
    (set `local.TempY` _index)
    (for _index_2 (range (`self.X`))
      (bind _output_get (set `local.TempX` _index_2))
      (bind _returnvalue_3 (`KismetMathLibrary.Conv_IntToDouble` _output_get))
      (`KismetArrayLibrary.Array_Add` _vertex2_2 (`KismetMathLibrary.MakeVector` _returnvalue_3 (`KismetMathLibrary.Conv_IntToDouble` _tempy_2)))
      (`KismetArrayLibrary.Array_Add` _vertex2_2 (`KismetMathLibrary.MakeVector` _returnvalue_3 (`KismetMathLibrary.Conv_IntToDouble` (+ _tempy_2 1))))
      (`KismetArrayLibrary.Array_Add` _vertex2_2 (`KismetMathLibrary.MakeVector` (`KismetMathLibrary.Conv_IntToDouble` (+ (`local.TempX`) 1)) (`KismetMathLibrary.Conv_IntToDouble` _tempy_2)))
      (`KismetArrayLibrary.Array_Add` _vertex2 (`KismetMathLibrary.MakeVector` (`KismetMathLibrary.Conv_IntToDouble` _tempx) (`KismetMathLibrary.Conv_IntToDouble` _returnvalue)))
      (`KismetArrayLibrary.Array_Add` _vertex2 (`KismetMathLibrary.MakeVector` _returnvalue_2 (`KismetMathLibrary.Conv_IntToDouble` _returnvalue)))
      (`KismetArrayLibrary.Array_Add` _vertex2 (`KismetMathLibrary.MakeVector` _returnvalue_2 (`KismetMathLibrary.Conv_IntToDouble` _tempy))))))

(fn `Spawn`
  (bind _proceduralmeshmanual (`self.ProceduralMeshManual`))
  (`KismetArrayLibrary.Array_Clear` (`self.Vertex2`))
  (`KismetArrayLibrary.Array_Clear` (`self.Triangles2`))
  (`KismetArrayLibrary.Array_Clear` (`self.UVs2`))
  (`self.CreateVertex`)
  (`self.CreateTriangles`)
  (`ProceduralMeshComponent.CreateMeshSection_LinearColor` :`self` _proceduralmeshmanual :`Vertices` (`self.Vertex2`) :`Triangles` (`self.Triangles2`))
  (`PrimitiveComponent.SetMaterial` _proceduralmeshmanual 0 null))

(fn `UserConstructionScript`
  (`self.Spawn`))