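; Player controller that streams BP_Chunk actors around the controlled pawn as it moves through the world.
; Tick compares the pawn's rounded grid coordinates with the last known ones, and a change triggers DestroyChunks, then SpawnNewChunk, which also runs at BeginPlay.
; Spawning fills missing cells within a circular radius, tracked in parallel coordinate and actor arrays.
; Destruction removes out-of-range entries during forward iteration, which can skip elements.
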(event `self.ReceiveBeginPlay`
  (`self.SpawnNewChunk`))

(event `self.ReceiveTick`
  (params (DeltaSeconds :type "Float (single-precision)"))
  (bind (_x _y) (`self.GetChunkCoords`))
  (bind (_x_2 _y_2) (`self.GetChunkCoords`))
  (bind (_lastknownchunkcoords_x _lastknownchunkcoords_y) (break `IntVector` (`self.LastKnownChunkCoords`)))
  (if (not (and (== _x_2 _lastknownchunkcoords_x) (== _y_2 _lastknownchunkcoords_y)))
    (set `self.LastKnownChunkCoords` (make `IntVector` _x _y))
    (`self.PlayerHasChangedChunkCords`)))

(event `PlayerHasChangedChunkCords`
  (`self.DestroyChunks`)
  (`self.SpawnNewChunk`))

(fn `DestroyChunks`
  (locals (ArrayIndex :type Integer))
  (bind _chunksize (`self.ChunkSIze`))
  (bind _currentspawnedchunkclasses (`self.CurrentSpawnedChunkClasses`))
  (bind _arrayindex (`local.ArrayIndex`))
  (for (_array_element _array_index) (`self.CurrentSpawnedChunkCoords`)
    (set `local.ArrayIndex` _array_index)
    (bind (_x _y) (break `IntVector` _array_element))
    (if (> (`KismetMathLibrary.Vector_Distance` (`KismetMathLibrary.MakeVector` (* _x _chunksize) (* _y _chunksize)) (`self.K2_GetActorLocation` (`self.K2_GetPawn`))) (* (`self.SpawnDistance`) (`self.ChunkSIze`)))
      (`self.K2_DestroyActor` (`|GetArrayItem` _currentspawnedchunkclasses _arrayindex))
      (`KismetArrayLibrary.Array_Remove` (`self.CurrentSpawnedChunkCoords`) _arrayindex)
      (`KismetArrayLibrary.Array_Remove` _currentspawnedchunkclasses _arrayindex))))

(fn `GetChunkCoords`
  (returns (X :type Integer) (Y :type Integer))
  (bind (_returnvalue_x _returnvalue_y) (`KismetMathLibrary.BreakVector` (/ (`self.K2_GetActorLocation` (`self.K2_GetPawn`)) (`self.ChunkSIze`))))
  (return (`KismetMathLibrary.Round` _returnvalue_x) (`KismetMathLibrary.Round` _returnvalue_y)))

(fn `SpawnNewChunk`
  (locals (`Temp X` :type Integer) (`Temp Y` :type Integer) (ChunkCoords :type "IntVector Structure"))
  (bind (_x _y) (`self.GetChunkCoords`))
  (bind _spawndistance (`self.SpawnDistance`))
  (bind _spawndistance_2 (`self.SpawnDistance`))
  (bind (_chunkcoords_x _chunkcoords_y) (break `IntVector` (`local.ChunkCoords`)))
  (bind _chunksize (`self.ChunkSIze`))
  (bind _temp_x (`local.Temp X`))
  (bind _temp_y (`local.Temp Y`))
  (bind _chunksize_2 (`self.ChunkSIze`))
  (for _index (range (* _spawndistance_2 -1) (+ _spawndistance_2 1))
    (set `local.Temp X` _index)
    (for _index_2 (range (* _spawndistance -1) (+ _spawndistance 1))
      (set `local.Temp Y` _index_2)
      (set `local.ChunkCoords` (make `IntVector` (+ _x _temp_x) (+ _y _temp_y)))
      (if (and (not (`KismetArrayLibrary.Array_Contains` (`self.CurrentSpawnedChunkCoords`) (`local.ChunkCoords`))) (<= (`KismetMathLibrary.VSize` (`KismetMathLibrary.MakeVector` (* _temp_x _chunksize_2) (* _temp_y _chunksize_2))) (* (`self.SpawnDistance`) (`self.ChunkSIze`))))
        (bind _returnvalue (`|SpawnActorFromClass` "/Game/BP_Chunk.BP_Chunk_C" (`KismetMathLibrary.MakeTransform` (`KismetMathLibrary.MakeVector` (* _chunkcoords_x _chunksize) (* _chunkcoords_y _chunksize))) "Undefined" "OverrideRootScale" null null))
        (`KismetArrayLibrary.Array_Add` (`self.CurrentSpawnedChunkCoords`) (`local.ChunkCoords`))
        (`KismetArrayLibrary.Array_Add` (`self.CurrentSpawnedChunkClasses`) _returnvalue)))))

(fn `UserConstructionScript`)